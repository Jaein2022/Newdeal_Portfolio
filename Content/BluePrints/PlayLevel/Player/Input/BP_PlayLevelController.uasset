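; BP_PlayLevelController is the play-level controller that sets up the player's Enhanced Input.
; On BeginPlay it adds the IMC_Player mapping context to the local player's input subsystem.
; An unconnected branch would spawn and store a VR or PC player pawn depending on whether a head-mounted display is enabled, but it never runs.
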(event Input|EnhancedActionEvents|EnhancedInputActionIA_Look_PC
  (params (ActionValue :type Vector%202D%20Structure) (ElapsedSeconds :type Float%20%28double-precision%29) (TriggeredSeconds :type Float%20%28double-precision%29) (InputAction :type Input%20Action%20Object%20Reference :default "/Game/BluePrints/PlayLevel/Player/Input/Action/PC/IA_Look_PC.IA_Look_PC")))

(event Input|EnhancedActionEvents|EnhancedInputActionIA_Shot_PC
  (params (ActionValue :type Boolean) (ElapsedSeconds :type Float%20%28double-precision%29) (TriggeredSeconds :type Float%20%28double-precision%29) (InputAction :type Input%20Action%20Object%20Reference :default "/Game/BluePrints/PlayLevel/Player/Input/Action/PC/IA_Shot_PC.IA_Shot_PC")))

(event Input|EnhancedActionEvents|EnhancedInputActionIA_Reload_PC
  (params (ActionValue :type Boolean) (ElapsedSeconds :type Float%20%28double-precision%29) (TriggeredSeconds :type Float%20%28double-precision%29) (InputAction :type Input%20Action%20Object%20Reference :default "/Game/BluePrints/PlayLevel/Player/Input/Action/PC/IA_Reload_PC.IA_Reload_PC")))

(event EventBeginPlay
  (Input|AddMappingContext (PlayerController|LocalPlayerSubsystems|GetEnhancedInputLocalPlayerSubsystem self) "/Game/BluePrints/PlayLevel/Player/Input/IMC_Player.IMC_Player" 0 "(bIgnoreAllPressedKeysUntilRelease=True,bForceImmediately=False)"))

(event EventTick
  (params (DeltaSeconds :type Float%20%28single-precision%29)))

(fn ConstructionScript)