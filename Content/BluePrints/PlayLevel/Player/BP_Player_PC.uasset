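; BP_Player_PC is the player pawn Blueprint, which handles first-person aiming with a rifle and no movement.
; On BeginPlay it spawns BP_Rifle, marks it equipped, and snaps it to the mesh's hand socket.
; It also snaps the camera to a head socket and registers the IMC_Default Enhanced Input mapping context.
; IA_Look drives controller yaw and pitch, and a TODO notes moving weapon handling to a weapon manager.
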(event Input|EnhancedActionEvents|EnhancedInputActionIA_Look
  (params (ActionValue :type Vector%202D%20Structure) (ElapsedSeconds :type Float%20%28double-precision%29) (TriggeredSeconds :type Float%20%28double-precision%29) (InputAction :type Input%20Action%20Object%20Reference :default "/Game/BluePrints/PlayLevel/Player/Input/Action/IA_Look.IA_Look"))
  ;[1 1 1] 플레이어 시점 회전. 이동은 하지 않으므로 구현하지 않음
  (:Triggered
    (Pawn|Input|AddControllerYawInput (.x ActionValue))
    (Pawn|Input|AddControllerPitchInput (.y ActionValue))))

(event EventBeginPlay
  ;[1 1 1] 시작시 무기를 소환하고 지정 위치에 고정. TODO 무기를 무기 매니저에서 관리(차후 확장을 위해)
  (|CallParentFunction)
  (bind _returnvalue (Game|SpawnActorfromClass "/Game/BluePrints/PlayLevel/Weapons/Rifle/BP_Rifle.BP_Rifle_C" (Math|Transform|MakeTransform "0, 0, 0" "0, 0, 0" "1.000000,1.000000,1.000000") "Undefined" self 0))
  (CallFunction|SetEquippedWeapon _returnvalue)
  (bind _equipedweapon (CallFunction|GetEquippedWeapon))
  (Default|SetEquipped _equipedweapon true)
  (Transformation|AttachComponentToComponent _equipedweapon (Variables|Default|GetSkeletalMesh) "hand_r_Weapon" "SnapToTarget" "SnapToTarget" "SnapToTarget" true)
  (Transformation|AttachComponentToComponent (Variables|Default|GetCamera) (Variables|Default|GetSkeletalMesh) "head_Camera" "SnapToTarget" "SnapToTarget" "SnapToTarget" true)
  (Input|AddMappingContext (PlayerController|LocalPlayerSubsystems|GetEnhancedInputLocalPlayerSubsystem (Game|GetPlayerController 0)) "/Game/BluePrints/PlayLevel/Player/Input/IMC_Default.IMC_Default" 0 "(bIgnoreAllPressedKeysUntilRelease=True,bForceImmediately=False)"))

(fn ConstructionScript
  (|CallParentFunction))