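; VR player pawn for the FPS play level, handling turning, shooting, weapon switching, magazine reloads, damage and death.
; Hand sphere traces pick weapons or magazines from body-mounted colliders, with WeaponRoot tracking camera XY at fixed height and ammo saved per weapon type.
; Reloading temporarily snaps the left hand to the weapon's magazine socket, then restores it to the controller.
; The attached menu swaps input mapping contexts and draws Niagara pointer beams from widget interactors.
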(event Custom|ReloadClientVR
  (bind _lefthand (Variables|Default|GetLeftHand))
  ;[0.1406 0.1406 0.1406] vr 리로드할때 왼손을 탄창에 붙였다가 애니메이션 끝날때 다시 모션컨트롤러에 붙이게
  (Variables|Default|SetbIsReloading true)
  (bind _grabmagazine (Variables|Default|GetGrabMagazine)
    (:then
      (Actor|DestroyActor _grabmagazine)
      (Variables|Default|SetbIsMagazineGrab false)
      (Transformation|DetachFromComponent _lefthand "KeepRelative" "KeepRelative" "KeepRelative" true)
      (bind _equipedweapon (CallFunction|GetEquippedWeapon))
      (Transformation|AttachComponentToComponent _lefthand (Variables|/Game/BluePrints/PlayLevel/Weapons/BP_Weapon.BP_Weapon_C|GetSkeletalMesh _equipedweapon) "Clip_Bone_GrabPos" "SnapToTarget" "SnapToTarget" "SnapToTarget" true)
      (Utilities|FlowControl|Delay 2.5)
      (Variables|Default|SetbIsReloading false)
      (Transformation|DetachFromComponent (Variables|Default|GetLeftHand) "KeepRelative" "KeepRelative" "KeepRelative" true)
      (Transformation|AttachComponentToComponent (Variables|Default|GetLeftHand) (Variables|Default|GetLeftMotionController) "None" "KeepRelative" "KeepRelative" "KeepRelative" true)
      (Transformation|SetRelativeTransform (Variables|Default|GetLeftHand) (Variables|Default|GetLeftHandRelativeTransform) false false))
    (:else)))

(event Custom|GetDamage
  (params (InDamage :type Integer))
  ;[0.1406 0.1406 0.1406] 피격
  (if (not (Variables|Default|GetbIsDead))
    (bind _output_get (Variables|Default|SetCurrentHP (- (Variables|Default|GetCurrentHP) InDamage)))
    (if (<= _output_get 0)
      (Audio|PlaySound2D "/Game/Audio/FX/169747__qubodup__dying-breath.169747__qubodup__dying-breath" 0.5 1.0 0.0 0 0)
      (Variables|Default|SetbIsDead true)
      (bind _asbp_play_level_controller (Utilities|Casting|CastToBP_PlayLevelController (Pawn|GetController)))
      (Class|EnhancedInputSubsystemInterface|ClearAllMappings(Message) _asbp_play_level_controller)
      (Transformation|DetachFromComponent (Variables|Default|GetLeftHand) "KeepRelative" "KeepRelative" "KeepRelative" true)
      (Transformation|DetachFromComponent (Variables|Default|GetRightHand) "KeepRelative" "KeepRelative" "KeepRelative" true)
      (bind _returnvalue (UserInterface|CreateWidget "/Game/UI/UI_GameResult.UI_GameResult_C"))
      (UserInterface|Viewport|AddtoViewport _returnvalue 0)
      (else
        (Default|ShowDamage (Variables|Default|GetUIDamage))
        (Audio|PlaySound2D "/Game/Audio/FX/437651__dersuperanton__damage-hit-voice-vocal.437651__dersuperanton__damage-hit-voice-vocal" 0.5 1.0 0.0 0 0)))))

(event Custom|SetWeapon
  (params (InWeapon :type BP%20Weapon%20Object%20Reference))
  ;[1 0.09375 0.09375] Weapon 변경 (GrabWeapon으로 변경하는방식으로 바뀔 예정)
  (Utilities|FlowControl|Sequence
    (:then_0
      (bind _equipedweapon (CallFunction|GetEquippedWeapon))
      (Utilities|IsValid _equipedweapon
        (:Is%20Valid
          (Default|SetEquipped _equipedweapon false)
          (Rendering|SetActorHiddenInGame _equipedweapon true)
          (Transformation|DetachFromActor _equipedweapon "KeepRelative" "KeepRelative" "KeepRelative")
          (Default|ResetWeaponUI (Variables|Default|GetUIDamage)))))
    (:then_1
      (Utilities|IsValid InWeapon
        (:Is%20Valid
          (CallFunction|SetEquippedWeapon InWeapon)
          (bind _equipedweapon_2 (CallFunction|GetEquippedWeapon))
          (Actor|SetOwner _equipedweapon_2 self)
          (Default|SetEquipped _equipedweapon_2 true)
          (Rendering|SetActorHiddenInGame _equipedweapon_2 false)
          (Transformation|AttachComponentToComponent _equipedweapon_2 (Variables|Default|GetRightHand) "hand_r_Weapon" "SnapToTarget" "SnapToTarget" "SnapToTarget" true)
          (switch Utilities|FlowControl|Switch|SwitchonE_WeaponType (Variables|/Game/BluePrints/PlayLevel/Weapons/BP_Weapon.BP_Weapon_C|GetWeaponType _equipedweapon_2)
            (:NewEnumerator0
              (Variables|Default|SetMagazineType "/Game/BluePrints/PlayLevel/Weapons/Magazine/BP_Magazine_Handgun.BP_Magazine_Handgun_C"))
            (:NewEnumerator1
              (Variables|Default|SetMagazineType "/Game/BluePrints/PlayLevel/Weapons/Magazine/BP_Magazine_Rifle.BP_Magazine_Rifle_C"))
            (:NewEnumerator2
              (Variables|Default|SetMagazineType "/Game/BluePrints/PlayLevel/Weapons/Magazine/BP_Magazine_RocketLauncher.BP_Magazine_RocketLauncher_C")))
          (Default|SetWeaponUI (Variables|Default|GetUIDamage) (Variables|/Game/BluePrints/PlayLevel/Weapons/BP_Weapon.BP_Weapon_C|GetWeaponType _equipedweapon_2))
          (CallFunction|SetRemainAmmoUI))))))

(event Input|EnhancedActionEvents|EnhancedInputActionIA_WeaponGrab
  (params (ActionValue :type Boolean) (ElapsedSeconds :type Float%20%28double-precision%29) (TriggeredSeconds :type Float%20%28double-precision%29) (InputAction :type Input%20Action%20Object%20Reference :default "/Game/BluePrints/PlayLevel/Player/Input/Action/VR/IA_WeaponGrab.IA_WeaponGrab"))
  (bind _righthand (Variables|Default|GetRightHand))
  (bind _returnvalue (Transformation|GetWorldLocation _righthand))
  (:Started
    (bind _outhit (Collision|SphereTraceByChannel _returnvalue _returnvalue 1e+01 "TraceTypeQuery6" false 0 "ForDuration" false))
    (CallFunction|GetGrabWeapon (.hitcomponent _outhit)))
  (:Completed
    (CallFunction|SetWeapon)))

(event Input|EnhancedActionEvents|EnhancedInputActionIA_MenuSelectLeft
  (params (ActionValue :type Boolean) (ElapsedSeconds :type Float%20%28double-precision%29) (TriggeredSeconds :type Float%20%28double-precision%29) (InputAction :type Input%20Action%20Object%20Reference :default "/Game/BluePrints/PlayLevel/Player/Input/Action/VR/IA_MenuSelectLeft.IA_MenuSelectLeft"))
  ;[0.4219 1 0.3112] MenuUI 연동
  (:Started
    (Class|WidgetInteractionComponent|PressPointerKey (Variables|Default|GetWidgetInteractionLeft) "LeftMouseButton"))
  (:Completed
    (Class|WidgetInteractionComponent|ReleasePointerKey (Variables|Default|GetWidgetInteractionLeft) "LeftMouseButton")))

(event Input|EnhancedActionEvents|EnhancedInputActionIA_Turn_VR
  (params (ActionValue :type Float%20%28double-precision%29) (ElapsedSeconds :type Float%20%28double-precision%29) (TriggeredSeconds :type Float%20%28double-precision%29) (InputAction :type Input%20Action%20Object%20Reference :default "/Game/BluePrints/PlayLevel/Player/Input/Action/VR/IA_Turn_VR.IA_Turn_VR"))
  ;[0.1406 0.1406 0.1406] VR 회전 이동. VR상에서 끊김현상 어떻게?
  (:Triggered
    (Class|Actor|AddActorWorldRotation (Math|Rotator|MakeRotator 0.0 0.0 (* ActionValue (Variables|Default|GetRotateSpeed) (Utilities|Time|GetWorldDeltaSeconds))))))

(event Input|EnhancedActionEvents|EnhancedInputActionIA_Shot_VR
  (params (ActionValue :type Boolean) (ElapsedSeconds :type Float%20%28double-precision%29) (TriggeredSeconds :type Float%20%28double-precision%29) (InputAction :type Input%20Action%20Object%20Reference :default "/Game/BluePrints/PlayLevel/Player/Input/Action/VR/IA_Shot_VR.IA_Shot_VR"))
  ;[0.1406 0.1406 0.1406] 사격
  (:Triggered
    (if (not (Variables|Default|GetbIsReloading))
      (bind _equipedweapon (CallFunction|GetEquippedWeapon))
      (Utilities|IsValid _equipedweapon
        (:Is%20Valid
          (Default|Shot _equipedweapon))))))

(event Input|EnhancedActionEvents|EnhancedInputActionIA_Pick_Magazine_VR
  (params (ActionValue :type Boolean) (ElapsedSeconds :type Float%20%28double-precision%29) (TriggeredSeconds :type Float%20%28double-precision%29) (InputAction :type Input%20Action%20Object%20Reference :default "/Game/BluePrints/PlayLevel/Player/Input/Action/VR/IA_Pick_Magazine_VR.IA_Pick_Magazine_VR"))
  (bind _lefthandaniminstance (Variables|Default|GetLeftHandAnimInstance))
  (bind _lefthandaniminstance_2 (Variables|Default|GetLeftHandAnimInstance))
  (bind _lefthand (Variables|Default|GetLeftHand))
  (bind _returnvalue (Transformation|GetWorldLocation _lefthand))
  ;[0.1406 0.1406 0.1406] 탄창 픽업
  (:Started
    (Variables|/Game/BluePrints/PlayLevel/Player/ABP_Player_VR_LeftHand.ABP_Player_VR_LeftHand_C|SetPoseAlphaGrasp (Variables|Default|GetLeftHandAnimInstance) 1.0)
    (bind _equipedweapon (CallFunction|GetEquippedWeapon))
    (Utilities|IsValid _equipedweapon
      (:Is%20Valid
        (bind _outhit (Collision|SphereTraceByChannel _returnvalue _returnvalue 1e+01 "TraceTypeQuery4" false 0 "ForDuration" false))
        (if (and (== (.hitcomponent _outhit) (Variables|Default|GetMagazine)) (> (Variables|Default|GetRemainAmmo) 0))
          (Variables|/Game/BluePrints/PlayLevel/Player/ABP_Player_VR_LeftHand.ABP_Player_VR_LeftHand_C|SetPoseAlphaGrasp _lefthandaniminstance_2 0.1)
          (Variables|/Game/BluePrints/PlayLevel/Player/ABP_Player_VR_LeftHand.ABP_Player_VR_LeftHand_C|SetPoseAlphaIndexCurl _lefthandaniminstance_2 0.1)
          (Variables|Default|SetbIsMagazineGrab true)
          (bind _returnvalue_2 (Game|SpawnActorfromClass (Variables|Default|GetMagazineType) (Math|Transform|MakeTransform "0, 0, 0" "0, 0, 0" "1.000000,1.000000,1.000000") "Undefined" self 0))
          (bind _output_get (Variables|Default|SetGrabMagazine _returnvalue_2))
          (Transformation|AttachComponentToComponent _output_get (Variables|Default|GetLeftHand) "hand_r_Magazine" "SnapToTarget" "SnapToTarget" "SnapToTarget" true)))))
  (:Completed
    (Variables|/Game/BluePrints/PlayLevel/Player/ABP_Player_VR_LeftHand.ABP_Player_VR_LeftHand_C|SetPoseAlphaGrasp _lefthandaniminstance 0.0)
    (Variables|/Game/BluePrints/PlayLevel/Player/ABP_Player_VR_LeftHand.ABP_Player_VR_LeftHand_C|SetPoseAlphaIndexCurl _lefthandaniminstance 0.0)
    (bind _grabmagazine (Variables|Default|GetGrabMagazine)
      (:then
        (Actor|DestroyActor _grabmagazine)
        (Variables|Default|SetbIsMagazineGrab false))
      (:else))))

(event Input|EnhancedActionEvents|EnhancedInputActionIA_Menu
  (params (ActionValue :type Float%20%28double-precision%29) (ElapsedSeconds :type Float%20%28double-precision%29) (TriggeredSeconds :type Float%20%28double-precision%29) (InputAction :type Input%20Action%20Object%20Reference :default "/Game/BluePrints/PlayLevel/Player/Input/Action/VR/IA_Menu.IA_Menu"))
  (bind _returnvalue (Game|GetPlayerController 0))
  (bind _returnvalue_2 (Game|GetPlayerController 0))
  (bind _returnvalue_3 (PlayerController|LocalPlayerSubsystems|GetEnhancedInputLocalPlayerSubsystem _returnvalue_2))
  (bind _returnvalue_4 (PlayerController|LocalPlayerSubsystems|GetEnhancedInputLocalPlayerSubsystem _returnvalue))
  ;[0.4219 1 0.3112] MenuUI 연동
  (:Started
    (if (Variables|Default|GetbMenu)
      (Variables|Default|SetbMenu false)
      (Rendering|SetVisibility (Variables|/Game/UI/Menu/BP_Menu.BP_Menu_C|GetDefaultSceneRoot (Variables|Default|GetMenuUI)) false true)
      (Input|RemoveMappingContext _returnvalue_4 "/Game/BluePrints/PlayLevel/Player/Input/IMC_Menu.IMC_Menu" "(bIgnoreAllPressedKeysUntilRelease=True,bForceImmediately=False)")
      (Input|AddMappingContext _returnvalue_4 "/Game/BluePrints/PlayLevel/Player/Input/IMC_Player.IMC_Player" 0 "(bIgnoreAllPressedKeysUntilRelease=True,bForceImmediately=False)")
      (Rendering|SetVisibility (Variables|Default|GetRightWidgetNiagara) false false)
      (Rendering|SetVisibility (Variables|Default|GetLeftWidgetNiagara) false false)
      (else
        (Variables|Default|SetbMenu true)
        (Rendering|SetVisibility (Variables|/Game/UI/Menu/BP_Menu.BP_Menu_C|GetDefaultSceneRoot (Variables|Default|GetMenuUI)) true true)
        (Input|RemoveMappingContext _returnvalue_3 "/Game/BluePrints/PlayLevel/Player/Input/IMC_Player.IMC_Player" "(bIgnoreAllPressedKeysUntilRelease=True,bForceImmediately=False)")
        (Input|AddMappingContext _returnvalue_3 "/Game/BluePrints/PlayLevel/Player/Input/IMC_Menu.IMC_Menu" 0 "(bIgnoreAllPressedKeysUntilRelease=True,bForceImmediately=False)")
        (Rendering|SetVisibility (Variables|Default|GetRightWidgetNiagara) true false)
        (Rendering|SetVisibility (Variables|Default|GetLeftWidgetNiagara) true false)))))

(event Input|EnhancedActionEvents|EnhancedInputActionIA_MenuSelectRight
  (params (ActionValue :type Boolean) (ElapsedSeconds :type Float%20%28double-precision%29) (TriggeredSeconds :type Float%20%28double-precision%29) (InputAction :type Input%20Action%20Object%20Reference :default "/Game/BluePrints/PlayLevel/Player/Input/Action/VR/IA_MenuSelectRight.IA_MenuSelectRight"))
  ;[0.4219 1 0.3112] MenuUI 연동
  (:Started
    (Class|WidgetInteractionComponent|PressPointerKey (Variables|Default|GetWidgetInteractionRight) "LeftMouseButton"))
  (:Completed
    (Class|WidgetInteractionComponent|ReleasePointerKey (Variables|Default|GetWidgetInteractionRight) "LeftMouseButton")))

(event EventBeginPlay
  (|CallParentFunction)
  (CallFunction|GetEquippedWeapon)
  (Class|HeadMountedDisplayFunctionLibrary|SetTrackingOrigin "Floor")
  ;[0.1406 0.1406 0.1406] Reload 이후 손의 위치를 원래대로 돌리기 위해 초기 상대좌표를 저장
  (Variables|Default|SetLeftHandRelativeTransform (Transformation|GetRelativeTransform (Variables|Default|GetLeftHand)))
  ;[0.1406 0.1406 0.1406] 왼손은 상황에따라 AnimInstance의 값이 바뀌어야하기 때문에 변수로 설정
  (bind _asabp_player_vr_left_hand (Utilities|Casting|CastToABP_Player_VR_LeftHand (Components|SkeletalMesh|GetAnimInstance (Variables|Default|GetLeftHand))))
  (bind _output_get (Variables|Default|SetLeftHandAnimInstance _asabp_player_vr_left_hand))
  (Variables|/Game/BluePrints/PlayLevel/Player/ABP_Player_VR_LeftHand.ABP_Player_VR_LeftHand_C|SetMirror _output_get true)
  (bind _asui_damage (Utilities|Casting|CastToUI_damage (UserInterface|GetWidget (Variables|Default|GetDamageWidget))))
  (Variables|Default|SetUIDamage _asui_damage)
  (bind _returnvalue (Game|SpawnActorfromClass "/Game/UI/Menu/BP_Menu.BP_Menu_C" (Math|Transform|MakeTransform "0, 0, 0" "0, 0, 0" "1.000000,1.000000,1.000000") "Undefined" 0 0))
  (bind _output_get_2 (Variables|Default|SetMenuUI _returnvalue))
  (Transformation|AttachComponentToComponent _output_get_2 (Variables|Default|GetMenuPos) "None" "SnapToTarget" "SnapToTarget" "SnapToTarget" true)
  (Rendering|SetVisibility (Variables|/Script/Engine.Actor|GetRootComponent _output_get_2) false true)
  (Utilities|Array|Resize (Variables|Default|GetAmmoArray) 3)
  (Utilities|Array|SetArrayElem (Variables|Default|GetAmmoArray) 0 9999)
  (Utilities|Array|SetArrayElem (Variables|Default|GetAmmoArray) 1 30)
  (Utilities|Array|SetArrayElem (Variables|Default|GetAmmoArray) 2 1)
  (Variables|Default|SetWeaponRootZPos (.z (Transformation|GetWorldLocation (Variables|Default|GetWeaponRoot)))))

(event EventTick
  (params (DeltaSeconds :type Float%20%28single-precision%29))
  (bind _camera (Variables|Default|GetCamera))
  (bind _returnvalue (Transformation|GetWorldLocation _camera))
  (Utilities|FlowControl|Sequence
    (:then_0
      (if (Variables|Default|GetbMenu)
        (CallFunction|WidgetTraceNiagara (Variables|Default|GetWidgetInteractionRight) (Variables|Default|GetRightWidgetNiagara))
        (CallFunction|WidgetTraceNiagara (Variables|Default|GetWidgetInteractionLeft) (Variables|Default|GetLeftWidgetNiagara))))
    (:then_1
      (Transformation|SetWorldLocation (Variables|Default|GetWeaponRoot) (Math|Vector|MakeVector (.x _returnvalue) (.y _returnvalue) (Variables|Default|GetWeaponRootZPos)) false false))))

(fn ConstructionScript
  (|CallParentFunction))

(fn Turn
  (params (RightTurn :type Boolean)))

(fn OnReload
  (|CallParentFunction)
  (CallFunction|ReloadClientVR))

(fn WidgetTraceNiagaraSystem
  (bind _leftarray (LocalVariables|GetLeftArray))
  (bind _widgetinteractionleft (Variables|Default|GetWidgetInteractionLeft))
  (Utilities|Array|Resize _leftarray 2)
  (Utilities|Array|SetArrayElem _leftarray 0 (Transformation|GetWorldLocation _widgetinteractionleft))
  (Utilities|Array|SetArrayElem (LocalVariables|GetLeftArray) 1 (* (Math|Vector|GetForwardVector _widgetinteractionleft) (Variables|/Script/UMG.WidgetInteractionComponent|GetInteractionDistance _widgetinteractionleft)))
  (Class|NiagaraDataInterfaceArrayFunctionLibrary|SetNiagaraArrayVector 0 "User.InPointArray" (LocalVariables|GetLeftArray)))

(fn GetGrabWeapon
  (params (InTraceComponent :type Primitive%20Component%20Object%20Reference))
  (Utilities|FlowControl|Sequence
    (:then_0
      (bind _equipedweapon (CallFunction|GetEquippedWeapon))
      (Utilities|IsValid _equipedweapon
        (:Is%20Valid
          (switch Utilities|FlowControl|Switch|SwitchonE_WeaponType (Variables|/Game/BluePrints/PlayLevel/Weapons/BP_Weapon.BP_Weapon_C|GetWeaponType _equipedweapon)
            (:NewEnumerator0
              (Utilities|Array|SetArrayElem (Variables|Default|GetAmmoArray) 0 (Variables|Default|GetRemainAmmo)))
            (:NewEnumerator1
              (Utilities|Array|SetArrayElem (Variables|Default|GetAmmoArray) 1 (Variables|Default|GetRemainAmmo)))
            (:NewEnumerator2
              (Utilities|Array|SetArrayElem (Variables|Default|GetAmmoArray) 2 (Variables|Default|GetRemainAmmo)))))))
    (:then_1
      (Utilities|FlowControl|Sequence
        (:then_0
          (if (== InTraceComponent (Variables|Default|GetHandGun))
            (LocalVariables|SetLocalWeaponType "NewEnumerator0")
            (bind _output_get (Variables|Default|SetRemainAmmo (Utilities|Array|Get(acopy) (Variables|Default|GetAmmoArray) (Math|Conversions|ToInteger(Byte) (LocalVariables|GetLocalWeaponType))) :!label _label))
            (Development|PrintString (Utilities|String|ToString(Integer) _output_get))
            (bind _bpgm_fps (CallFunction|GetGameModeFPS))
            (bind _gamemanager (Default|GetGameManager _bpgm_fps))
            (bind _weaponmanager (Default|GetWeaponManager _gamemanager))
            (Default|SetWeaponbyType _weaponmanager (LocalVariables|GetLocalWeaponType))
            (return)))
        (:then_1
          (if (== InTraceComponent (Variables|Default|GetRifleCol))
            (LocalVariables|SetLocalWeaponType "NewEnumerator1")
            (goto _label)))
        (:then_2
          (if (== InTraceComponent (Variables|Default|GetRocketLauncherCol))
            (LocalVariables|SetLocalWeaponType "NewEnumerator2")
            (goto _label)))))))

(fn CalcWeaponRootPos
  (bind _weaponroot (Variables|Default|GetWeaponRoot))
  (bind _returnvalue (Transformation|GetWorldRotation _weaponroot))
  (Transformation|SetWorldRotation _weaponroot (Math|Rotator|MakeRotator (.roll _returnvalue) (.pitch _returnvalue) (.yaw (Transformation|GetWorldRotation (Variables|Default|GetCamera)))) false false))

(fn WidgetTraceNiagara
  (params (InWidgetInteraction :type Widget%20Interaction%20Component%20Object%20Reference) (InNiagaraSystem :type Niagara%20Component%20Object%20Reference))
  (bind _localpointarray (LocalVariables|GetLocalPointArray))
  (bind _returnvalue (Transformation|GetWorldLocation InWidgetInteraction))
  (Utilities|Array|Resize _localpointarray 2)
  (Utilities|Array|SetArrayElem _localpointarray 0 _returnvalue)
  (Utilities|Array|SetArrayElem (LocalVariables|GetLocalPointArray) 1 (+ (* (Class|KismetMathLibrary|MatrixGetUnitAxis (Math|Transform|ToMatrix(Transform) (Transformation|GetWorldTransform InWidgetInteraction)) "X") (Variables|/Script/UMG.WidgetInteractionComponent|GetInteractionDistance InWidgetInteraction)) _returnvalue))
  (Class|NiagaraDataInterfaceArrayFunctionLibrary|SetNiagaraArrayVector InNiagaraSystem "User.InPointArray" (LocalVariables|GetLocalPointArray)))

(fn SetRemainAmmoUI
  (bind _equipedweapon (CallFunction|GetEquippedWeapon))
  (Utilities|IsValid _equipedweapon
    (:Is%20Valid
      (Rendering|Components|TextRender|SetText (Variables|/Game/UI/UI_damage.UI_damage_C|GetRemainAmmo (Variables|Default|GetUIDamage)) (Utilities|Text|ToText(Integer) (Variables|Default|GetRemainAmmo))))
    (:Is%20Not%20Valid
      (Rendering|Components|TextRender|SetText (Variables|/Game/UI/UI_damage.UI_damage_C|GetRemainAmmo (Variables|Default|GetUIDamage)) ""))))