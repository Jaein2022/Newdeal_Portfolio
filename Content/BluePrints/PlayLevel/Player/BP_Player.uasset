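; FPS player Blueprint that handles shooting, reloading, reserve ammo, health and death state.
; Shoot and reload inputs call the equipped weapon and play montages, with reload gated on remaining ammo and reload state.
; SetRemainAmmo subtracts used ammo, clamps at zero and updates the GameMode's AmmoUI.
; GetDamage and OnDamaged duplicate HP, hit montage, sound and death logic; only GetDamage also triggers the damage widget.
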(event Custom|GetDamage
  (params (InDamage :type Integer))
  (if (not (Variables|Default|GetbIsDead))
    (bind _output_get (Variables|Default|SetCurrentHP (- (Variables|Default|GetCurrentHP) InDamage)))
    (if (<= _output_get 0)
      (Audio|PlaySound2D "/Game/Audio/FX/169747__qubodup__dying-breath.169747__qubodup__dying-breath" 0.5 1.0 0.0 0 0)
      (Variables|Default|SetbIsDead true)
      (else
        (bind _asui_damage (Utilities|Casting|CastToUI_damage (UserInterface|GetWidget (Variables|Default|GetDamageUI)))
          (:then
            (Default|ShowDamage1 _asui_damage)
            (Animation|Montage|PlayMontage (Variables|Default|GetSkeletalMesh) (Variables|Default|GetHitAnimMontage)
              (:then
                (Audio|PlaySound2D "/Game/Audio/FX/437651__dersuperanton__damage-hit-voice-vocal.437651__dersuperanton__damage-hit-voice-vocal" 0.5 1.0 0.0 0 0))))
          (:CastFailed
            (Development|PrintText "Hello")))))))

(event Input|EnhancedActionEvents|EnhancedInputActionIA_Reload
  (params (ActionValue :type Boolean) (ElapsedSeconds :type Float%20%28double-precision%29) (TriggeredSeconds :type Float%20%28double-precision%29) (InputAction :type Input%20Action%20Object%20Reference :default "/Game/BluePrints/PlayLevel/Player/Input/Action/IA_Reload.IA_Reload"))
  ;[0.1406 0.1406 0.1406] 남은 탄이 있다면 재장전
  (:Started
    (if (and (> (Variables|Default|GetRemainAmmo) 0) (not (Variables|Default|GetbIsReloading)))
      (Default|Reload (Variables|Default|GetEquippedWeapon))
      (Animation|Montage|PlayMontage (Variables|Default|GetSkeletalMesh) (Variables|Default|GetReloadAnimMontage)))))

(event Input|EnhancedActionEvents|EnhancedInputActionIA_Shoot
  (params (ActionValue :type Boolean) (ElapsedSeconds :type Float%20%28double-precision%29) (TriggeredSeconds :type Float%20%28double-precision%29) (InputAction :type Input%20Action%20Object%20Reference :default "/Game/BluePrints/PlayLevel/Player/Input/Action/IA_Shoot.IA_Shoot"))
  ;[0.1406 0.1406 0.1406] 장비된 무기가 있다면 shot 함수 호출
  (:Triggered
    (bind _equippedweapon (Variables|Default|GetEquippedWeapon)
      (:then
        (Default|Shot _equippedweapon)
        (Animation|Montage|PlayMontage (Variables|Default|GetSkeletalMesh) (Variables|Default|GetShotAnimMontage)))
      (:else))))

(event EventBeginPlay
  ;[1 0.09896 0.09896] 총알수 확인용 임시 사용 나중에 지울것임
  (bind _asbpgm_fps (Utilities|Casting|CastToBPGM_FPS (Game|GetGameMode)))
  (Rendering|Components|TextRender|SetText (Variables|/Game/BluePrints/PlayLevel/Player/UI/WB_AmmoSample.WB_AmmoSample_C|GetRemainAmmo (Variables|/Game/BluePrints/PlayLevel/BPGM_FPS.BPGM_FPS_C|GetAmmoUI _asbpgm_fps)) (Utilities|Text|ToText(Integer) (Variables|Default|GetRemainAmmo)))
  (bind _asui_damage (Utilities|Casting|CastToUI_damage (UserInterface|GetWidget (Variables|Default|GetDamageUI)))
    (:then
      (UserInterface|Viewport|AddtoViewport _asui_damage 0))
    (:CastFailed
      (Development|PrintText "Hello"))))

(event Collision|EventActorBeginOverlap
  (params (OtherActor :type Actor%20Object%20Reference)))

(event EventTick
  (params (DeltaSeconds :type Float%20%28single-precision%29)))

(fn ConstructionScript)

(fn GetRemainAmmo
  (return (Variables|Default|GetRemainAmmo)))

(fn SetRemainAmmo
  (params (InUseAmmo :type Integer))
  (bind _output_get (Variables|Default|SetRemainAmmo (- (Variables|Default|GetRemainAmmo) InUseAmmo)))
  (if (< _output_get 0)
    (Variables|Default|SetRemainAmmo 0))
  (bind _asbpgm_fps (Utilities|Casting|CastToBPGM_FPS (Game|GetGameMode)))
  (Rendering|Components|TextRender|SetText (Variables|/Game/BluePrints/PlayLevel/Player/UI/WB_AmmoSample.WB_AmmoSample_C|GetRemainAmmo (Variables|/Game/BluePrints/PlayLevel/BPGM_FPS.BPGM_FPS_C|GetAmmoUI _asbpgm_fps)) (Utilities|Text|ToText(Integer) (Variables|Default|GetRemainAmmo))))

(fn GetIsAttacking
  (return (Variables|Default|GetbIsAttacking)))

(fn SetIsAttacking
  (params (InIsAttacking :type Boolean))
  (Variables|Default|SetbIsAttacking InIsAttacking))

(fn GetEquippedWeapon
  (return (Variables|Default|GetEquippedWeapon)))

(fn SetEquippedWeapon
  (params (InEquippedWeapon :type BP%20Weapon%20Object%20Reference))
  (Variables|Default|SetEquippedWeapon InEquippedWeapon))

(fn GetMaxHP
  (return (Variables|Default|GetMaxHP)))

(fn SetMaxHP
  (params (InMaxHP :type Integer))
  (Variables|Default|SetMaxHP InMaxHP))

(fn GetCurrentHP
  (return (Variables|Default|GetCurrentHP)))

(fn SetCurrnetHP
  (params (InCurrentHP :type Integer))
  (Variables|Default|SetCurrentHP InCurrentHP))

(fn SetIsReloading
  (params (InIsReloading :type Boolean))
  (Variables|Default|SetbIsReloading InIsReloading))

(fn GetIsDead
  (return (Variables|Default|GetbIsDead)))

(fn OnDamaged
  (params (InDamage :type Integer))
  (if (not (Variables|Default|GetbIsDead))
    (bind _output_get (Variables|Default|SetCurrentHP (- (Variables|Default|GetCurrentHP) InDamage)))
    (if (<= _output_get 0)
      (Audio|PlaySound2D "/Game/Audio/FX/169747__qubodup__dying-breath.169747__qubodup__dying-breath" 0.5 1.0 0.0 0 0)
      (Variables|Default|SetbIsDead true)
      (else
        (Animation|Montage|MontagePlay (Components|SkeletalMesh|GetAnimInstance (Variables|Default|GetSkeletalMesh)) (Variables|Default|GetHitAnimMontage) 1.0 "MontageLength" 0.0 true)
        (Audio|PlaySound2D "/Game/Audio/FX/437651__dersuperanton__damage-hit-voice-vocal.437651__dersuperanton__damage-hit-voice-vocal" 0.5 1.0 0.0 0 0)))))