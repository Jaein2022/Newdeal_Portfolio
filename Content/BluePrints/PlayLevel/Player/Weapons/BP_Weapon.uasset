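; BP_Weapon is the player's FPS firearm, handling firing, reloading and a laser sight.
; Shot spends ammo, plays the fire montage, ejects a casing, shakes the camera and runs a debug-drawn line trace whose hit is unused, then waits out a fire delay.
; Reload refills from reserve ammo on montage completion and reports the amount to BP_Player; ammo changes update the game mode's UI.
; Tick feeds barrel-forward endpoints to a Niagara laser.
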(event Custom|Shot
  (bind _barralpoint (Variables|Default|GetBarralPoint))
  (bind _cartridgecasepoint (Variables|Default|GetCartridgeCasePoint))
  (bind _returnvalue (Transformation|GetWorldLocation _barralpoint))
  (bind _returnvalue_2 (Transformation|GetWorldTransform _cartridgecasepoint))
  (if (Math|Boolean|ANDBoolean (Variables|Shot|GetbEquiped) (Variables|Shot|GetbCanShot) (> (Variables|Shot|GetCurrentAmmo) 0) (not (Variables|Shot|GetbIsReloading)))
    (Math|Integer|DecrementInt (Variables|Shot|GetCurrentAmmo)
      (:%20%20
        (CallFunction|UpdateCurrentAmmo)
        (Animation|Montage|PlayMontage (Variables|Default|GetSkeletalMesh) (Variables|Default|GetFireMontage)
          (:then
            (Game|SpawnActorfromClass (Variables|Default|GetcCartridgeCase) (Math|Transform|MakeTransform (.location _returnvalue_2) (.rotation _returnvalue_2) "1.000000,1.000000,1.000000") "Undefined" 0 0)
            (Camera|PlayWorldCameraShake "/Game/BluePrints/PlayLevel/Player/Weapons/BP_CameraShake.BP_CameraShake_C" (Transformation|GetActorLocation) 0.0 2e+02)
            (Collision|LineTraceByChannel _returnvalue (+ _returnvalue (* (Math|Vector|GetForwardVector (Transformation|GetWorldRotation _barralpoint)) 2e+03)) "TraceTypeQuery3" false 0 "ForDuration")
            (Variables|Shot|SetbCanShot false)
            (Utilities|FlowControl|Delay (Variables|Shot|GetDelay))
            (Variables|Shot|SetbCanShot true)))))))

(event Custom|Reload
  (params (InRemainAmmo :type Integer))
  (if (not (Variables|Shot|GetbIsReloading))
    (Variables|Shot|SetNeedAmmo (- (Variables|Shot|GetMaxAmmo) (Variables|Shot|GetCurrentAmmo)))
    (if (> (Variables|Shot|GetNeedAmmo) 0)
      (Variables|Shot|SetbIsReloading true)
      (Animation|Montage|PlayMontage (Variables|Default|GetSkeletalMesh) (Variables|Default|GetReloadMontage)
        (:OnCompleted
          (if (> InRemainAmmo (Variables|Shot|GetNeedAmmo))
            (Variables|Shot|SetCurrentAmmo (Variables|Shot|GetMaxAmmo))
            (Default|SetRemainAmmo (Variables|Default|GetOwnerPlayer) (Variables|Shot|GetNeedAmmo))
            (else
              (Variables|Shot|SetCurrentAmmo (+ (Variables|Shot|GetCurrentAmmo) InRemainAmmo))
              (Default|SetRemainAmmo (Variables|Default|GetOwnerPlayer) InRemainAmmo)))
          (Variables|Shot|SetbIsReloading false)
          (CallFunction|UpdateCurrentAmmo))))))

(event EventBeginPlay
  (bind _asbp_player (Utilities|Casting|CastToBP_Player (Components|GetOwner)))
  (Variables|Default|SetOwnerPlayer _asbp_player)
  (CallFunction|UpdateCurrentAmmo)
  (Utilities|Array|Resize (Variables|Default|GetLaserPointerArray) 2))

(event EventTick
  (params (DeltaSeconds :type Float%20%28single-precision%29))
  (CallFunction|LaserPointer))

(fn ConstructionScript)

(fn UpdateCurrentAmmo
  (bind _asbpgm_fps (Utilities|Casting|CastToBPGM_FPS (Game|GetGameMode)))
  (Rendering|Components|TextRender|SetText (Variables|/Game/BluePrints/PlayLevel/Player/UI/WB_AmmoSample.WB_AmmoSample_C|GetCurrentAmmo (Variables|/Game/BluePrints/PlayLevel/BPGM_FPS.BPGM_FPS_C|GetAmmoUI _asbpgm_fps)) (Utilities|Text|ToText(Integer) (Variables|Shot|GetCurrentAmmo))))

(fn LaserPointer
  (bind _barralpoint (Variables|Default|GetBarralPoint))
  (bind _returnvalue (Transformation|GetWorldLocation _barralpoint))
  (Utilities|Array|SetArrayElem (Variables|Default|GetLaserPointerArray) 0 _returnvalue)
  (Utilities|Array|SetArrayElem (Variables|Default|GetLaserPointerArray) 1 (+ _returnvalue (* (Math|Vector|GetForwardVector (Transformation|GetWorldRotation (Variables|Default|GetBarralPoint))) 1e+03)))
  (Class|NiagaraDataInterfaceArrayFunctionLibrary|SetNiagaraArrayVector (Variables|Default|GetLaserPointerNiagaraSystem) "User.InPointArray" (Variables|Default|GetLaserPointerArray)))