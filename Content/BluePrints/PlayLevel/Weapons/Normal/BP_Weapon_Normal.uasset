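; BP_Weapon_Normal is a hitscan gun with a Niagara laser pointer, extending a parent weapon class.
; OnShot ejects a short-lived cartridge case, then line-traces from the barrel and damages hit enemies, flagging headshots by "Head" in the component name.
; Each tick, a separate-channel trace spawns an impact effect on hits and feeds a Niagara position array, drawing only the last fifth of the beam.
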(event EventBeginPlay
  (|CallParentFunction)
  (Utilities|Array|Resize (Variables|Default|GetLaserPointerArray) 2))

(event Collision|EventActorBeginOverlap
  (params (OtherActor :type Actor%20Object%20Reference)))

(event EventTick
  (params (DeltaSeconds :type Float%20%28single-precision%29))
  (|CallParentFunction DeltaSeconds)
  (CallFunction|LaserPointer))

(fn ConstructionScript
  (|CallParentFunction))

(fn OnShot
  (bind _catridgecasepoint (Variables|Default|GetCatridgeCasePoint))
  (bind _barralpoint (Variables|Default|GetBarralPoint))
  (bind _returnvalue (Transformation|GetWorldLocation _barralpoint))
  (bind _returnvalue_2 (Transformation|GetWorldTransform _catridgecasepoint))
  (|CallParentFunction)
  ;[0.1406 0.1406 0.1406] 탄피
  (bind _returnvalue_3 (Game|SpawnActorfromClass (Variables|Default|GetcCartridgeCase) (Math|Transform|MakeTransform (.location _returnvalue_2) (.rotation _returnvalue_2) "1.000000,1.000000,1.000000") "Undefined" 0 0))
  (Actor|SetLifeSpan _returnvalue_3 1.0)
  ;[0.1406 0.1406 0.1406] 타격 부위에 따른 데미지 계산
  (bind _outhit (Collision|LineTraceByChannel _returnvalue (+ _returnvalue (* (Math|Vector|GetForwardVector (Transformation|GetWorldRotation _barralpoint)) 2e+03)) "TraceTypeQuery3" false 0 "None"))
  (bind _asbp_enemy_character_base (Utilities|Casting|CastToBP_EnemyCharacter_Base (.hitactor _outhit)))
  (Default|OnDamaged _asbp_enemy_character_base (Variables|Default|GetAttack) (Utilities|String|Contains (Utilities|GetDisplayName (.hitcomponent _outhit)) "Head") false))

(fn LaserPointer
  (bind _barralpoint (Variables|Default|GetBarralPoint))
  (bind _returnvalue (Transformation|GetWorldLocation _barralpoint))
  ;[0.1406 0.1406 0.1406] 레이저 포인터 업데이트용
  (LocalVariables|SetLocalLaserStartPoint _returnvalue)
  (LocalVariables|SetLocalLaserEndPoint (+ _returnvalue (* (Math|Vector|GetForwardVector (Transformation|GetWorldRotation (Variables|Default|GetBarralPoint))) 2e+03)))
  (Utilities|FlowControl|Sequence
    (:then_0
      (bind (_outhit _returnvalue_2) (Collision|LineTraceByChannel (LocalVariables|GetLocalLaserStartPoint) (LocalVariables|GetLocalLaserEndPoint) "TraceTypeQuery5" false 0 "None"))
      (if _returnvalue_2
        (bind _output_get (LocalVariables|SetLocalLaserEndPoint (.impactpoint _outhit)))
        (Niagara|SpawnSystematLocation "/Game/BluePrints/PlayLevel/Player/VFX/NS_LaserEnd.NS_LaserEnd" _output_get)))
    (:then_1
      (LocalVariables|SetLocalLaserStartPoint (- (LocalVariables|GetLocalLaserEndPoint) (* (Math|Vector|GetForwardVector (Transformation|GetWorldRotation (Variables|Default|GetBarralPoint))) (* (Math|Vector|Distance(Vector) (LocalVariables|GetLocalLaserEndPoint) (LocalVariables|GetLocalLaserStartPoint)) 0.2))))
      (Utilities|Array|SetArrayElem (Variables|Default|GetLaserPointerArray) 0 (LocalVariables|GetLocalLaserStartPoint))
      (Utilities|Array|SetArrayElem (Variables|Default|GetLaserPointerArray) 1 (LocalVariables|GetLocalLaserEndPoint))
      (Class|NiagaraDataInterfaceArrayFunctionLibrary|SetNiagaraArrayVector (Variables|Default|GetLaserPointerParticleSystem) "User.InPointArray" (Variables|Default|GetLaserPointerArray)))))