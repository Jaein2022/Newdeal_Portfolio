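; Base VR weapon Blueprint that handles firing, reloading and the on-weapon ammo widget for BP_Player_VR.
; Shot checks equip, cooldown and reload state, then spends a round, plays a montage and camera shake, and calls the empty OnShot hook, or dry-fires when empty.
; Reload plays a montage, refills from the player's reserve on completion and updates both ammo UIs.
; When reserve is short, Hand Gun skips the reserve deduction.
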(event Custom|Shot
  ;[0.1406 0.1406 0.1406] 사격
  ;;[0.1406 0.1406 0.1406] 사격조건(장비중이고, 사격가능한 상태이고, 총알이 있고, 재장전 중이 아닐때)
  (if (Math|Boolean|ANDBoolean (Variables|Shot|GetbEquipped) (Variables|Shot|GetbCanShot) (not (Variables|Shot|GetbIsReloading)))
    (if (> (Variables|Shot|GetCurrentAmmo) 0)
      (Utilities|FlowControl|Sequence
        (:then_0
          (Math|Integer|DecrementInt (Variables|Shot|GetCurrentAmmo)
            (:%20%20
              (Animation|Montage|PlayMontage (Variables|Default|GetSkeletalMesh) (Variables|Default|GetFireMontage)
                (:then
                  (CallFunction|OnShot)
                  (Camera|PlayWorldCameraShake "/Game/BluePrints/PlayLevel/Weapons/BP_CameraShake_Shot.BP_CameraShake_Shot_C" (Transformation|GetActorLocation) 0.0 2e+02)
                  (CallFunction|SetAmmoUI))))))
        (:then_1
          (Variables|Shot|SetbCanShot false)
          (Utilities|FlowControl|Delay (Variables|Shot|GetDelay))
          (Variables|Shot|SetbCanShot true)))
      (elif (not (Variables|Default|GetbDryShotSoundPlay))
        (Audio|PlaySoundatLocation (Variables|Default|GetDryFireSound) (Transformation|GetActorLocation) "0, 0, 0" 1.0 1.0 0.0 0 0 0 0)
        (Variables|Default|SetbDryShotSoundPlay true)
        (Utilities|FlowControl|Delay (Variables|Shot|GetDelay))
        (Variables|Default|SetbDryShotSoundPlay false)))))

(event Custom|SetAmmoUI
  (bind _uiweaponammo (Variables|Default|GetUIWeaponAmmo))
  (Rendering|Components|TextRender|SetText (Variables|/Game/UI/UI_WeaponAmmo.UI_WeaponAmmo_C|GetCurrent _uiweaponammo) (Utilities|Text|ToText(Integer) (Variables|Shot|GetCurrentAmmo)))
  (Rendering|Components|TextRender|SetText (Variables|/Game/UI/UI_WeaponAmmo.UI_WeaponAmmo_C|GetMax _uiweaponammo) (Utilities|Text|ToText(Integer) (Variables|Shot|GetMaxAmmo))))

(event Custom|Reload
  (bind _ownerplayer (Variables|Default|GetOwnerPlayer))
  ;[0.1406 0.1406 0.1406] 재장전, 플레이어로 부터 현재 남아있는 전체 탄환을 받아온 후, 자신이 필요한 탄환수와 비교해서 필요한 만큼만 차감시킴
  (if (not (Variables|Shot|GetbIsReloading))
    (Variables|Shot|SetNeedAmmo (- (Variables|Shot|GetMaxAmmo) (Variables|Shot|GetCurrentAmmo)))
    (if (> (Variables|Shot|GetNeedAmmo) 0)
      (bind _output_get (Variables|Shot|SetbIsReloading true))
      (Default|SetIsReloading (Variables|Default|GetOwnerPlayer) _output_get)
      (Animation|Montage|PlayMontage (Variables|Default|GetSkeletalMesh) (Variables|Default|GetReloadMontage)
        (:then
          (bind _asbp_player_vr (Utilities|Casting|CastToBP_Player_VR (Variables|Default|GetOwnerPlayer)))
          (Default|ReloadClientVR _asbp_player_vr))
        (:OnCompleted
          (bind _outremainammo (Default|GetRemainAmmo (Variables|Default|GetOwnerPlayer)))
          (if (> _outremainammo (Variables|Shot|GetNeedAmmo))
            ;;[0.1406 0.1406 0.1406] 플레이어에게 남은 탄이 충분하면 최대치로 재장전
            (Variables|Shot|SetCurrentAmmo (Variables|Shot|GetMaxAmmo))
            (Default|SetRemainAmmo (Variables|Default|GetOwnerPlayer) (Variables|Shot|GetNeedAmmo))
            (else
              ;;[0.1406 0.1406 0.1406] 플레이어에게 남은 탄이 더 부족하면 플레이어에게 있는 만큼만 재장전
              (Variables|Shot|SetCurrentAmmo (+ (Variables|Shot|GetCurrentAmmo) _outremainammo))
              (switch Utilities|FlowControl|Switch|SwitchonE_WeaponType (Variables|Default|GetWeaponType)
                (:NewEnumerator0
                  _)
                (:NewEnumerator1
                  (Default|SetRemainAmmo (Variables|Default|GetOwnerPlayer) _outremainammo :!label _label))
                (:NewEnumerator2
                  (goto _label)))))
          (bind _output_get_2 (Variables|Shot|SetbIsReloading false))
          (Default|SetIsReloading _ownerplayer _output_get_2)
          (CallFunction|SetAmmoUI)
          (bind _asbp_player_vr_2 (Utilities|Casting|CastToBP_Player_VR _ownerplayer))
          (Default|SetRemainAmmoUI _asbp_player_vr_2))))))

(event EventBeginPlay
  (bind _asbp_player_vr (Utilities|Casting|CastToBP_Player_VR (Game|Player|GetPlayerPawn 0)))
  (Variables|Default|SetOwnerPlayer _asbp_player_vr)
  (bind _asui_weapon_ammo (Utilities|Casting|CastToUI_WeaponAmmo (UserInterface|GetWidget (Variables|Default|GetAmmoWidget))))
  (Variables|Default|SetUIWeaponAmmo _asui_weapon_ammo)
  (CallFunction|SetAmmoUI))

(fn ConstructionScript)

(fn GetEquipped
  (return (Variables|Shot|GetbEquipped)))

(fn SetEquipped
  (params (InEquipped :type Boolean))
  (Variables|Shot|SetbEquipped InEquipped))

(fn GetCurrentAmmo
  (return (Variables|Shot|GetCurrentAmmo)))

(fn SetCurrentAmmo
  (params (InCurrentAmmo :type Integer))
  (Variables|Shot|SetCurrentAmmo InCurrentAmmo))

(fn SetOwnerPlayer
  (params (InPlayer :type BP%20Player%20Object%20Reference))
  (Variables|Default|SetOwnerPlayer InPlayer))

(fn OnShot)