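; Base launcher projectile that explodes on impact or when its short lifespan expires, damaging enemies and the VR player.
; Tick runs a small sphere trace at its location and destroys the actor on any hit, leaving the overlap events empty.
; The Destroyed event spawns a rocket explosion actor, applies explosion damage to enemies found by a debug-drawn ExplosionRange sphere trace, and hurts the player through a separate distance check.
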(event OnComponentBeginOverlap(Sphere)
  (params (OverlappedComponent :type Primitive%20Component%20Object%20Reference) (OtherActor :type Actor%20Object%20Reference) (OtherComp :type Primitive%20Component%20Object%20Reference) (OtherBodyIndex :type Integer) (bFromSweep :type Boolean) (SweepResult :type Hit%20Result%20Structure%20%28by%20ref%29)))

(event EventBeginPlay
  (Actor|SetLifeSpan 3.0))

(event Collision|EventActorBeginOverlap
  (params (OtherActor :type Actor%20Object%20Reference)))

(event EventTick
  (params (DeltaSeconds :type Float%20%28single-precision%29))
  (bind _returnvalue (Transformation|GetActorLocation))
  (bind _returnvalue_2 (Collision|MultiSphereTraceByChannel _returnvalue _returnvalue 15.0 "TraceTypeQuery5" false 0 "None"))
  (if _returnvalue_2
    (Actor|DestroyActor)))

(event EventDestroyed
  (bind _returnvalue (Transformation|GetActorLocation))
  (Game|SpawnActorfromClass "/Game/BluePrints/PlayLevel/Weapons/Launcher/RocketLauncher/BP_RocketLauncherExplosion.BP_RocketLauncherExplosion_C" (Transformation|GetActorTransform) "Undefined" 0 0)
  (bind _outhits (Collision|MultiSphereTraceByChannel _returnvalue _returnvalue (Variables|Default|GetExplosionRange) "TraceTypeQuery3" false 0 "ForDuration"))
  (for _array_element _outhits
    (bind _asbp_enemy_character_base (Utilities|Casting|CastToBP_EnemyCharacter_Base (.hitactor _array_element)))
    (Default|OnDamaged _asbp_enemy_character_base 15 false true "0, 0, 0"))
  (bind _asbp_player_vr (Utilities|Casting|CastToBP_Player_VR (Game|Player|GetPlayerPawn 0)))
  (if (<= (Math|Vector|Distance(Vector) (Transformation|GetActorLocation) (Transformation|GetActorLocation _asbp_player_vr)) (Variables|Default|GetExplosionRange))
    (Default|GetDamage _asbp_player_vr 50))
  (Actor|DestroyActor))

(fn ConstructionScript)