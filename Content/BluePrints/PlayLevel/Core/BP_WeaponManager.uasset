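; BP_WeaponManager is an actor that owns the pool of weapons and cycles them on the VR player.
; On BeginPlay it spawns one actor per DT_Weapon row into a Weapons array and caches the BP_Player_VR pawn.
; Each SetWeapon call hands the weapon at NextWeaponIndex to the player, then advances the index, wrapping to the first after the last.
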(event EventBeginPlay
  (CallFunction|InitWeapons)
  (bind _asbp_player_vr (Utilities|Casting|CastToBP_Player_VR (Game|Player|GetPlayerPawn 0)))
  (Variables|Default|SetPlayer _asbp_player_vr))

(event Collision|EventActorBeginOverlap
  (params (OtherActor :type Actor%20Object%20Reference)))

(event EventTick
  (params (DeltaSeconds :type Float%20%28single-precision%29)))

(fn ConstructionScript)

(fn InitWeapons
  (bind _outrownames (DataTable|GetDataTableRowNames "/Game/BluePrints/PlayLevel/Weapons/DT_Weapon.DT_Weapon"))
  (for _array_element _outrownames
    (bind _returnvalue (Utilities|GetDataTableRow "/Game/BluePrints/PlayLevel/Weapons/DT_Weapon.DT_Weapon" _array_element)
      (:then
        (bind _returnvalue_2 (Game|SpawnActorfromClass (.weapon _returnvalue) (Math|Transform|MakeTransform "0, 0, 0" "0, 0, 0" "1.000000,1.000000,1.000000") "Undefined" 0 0))
        (Utilities|Array|Add (Variables|Default|GetWeapons) _returnvalue_2)))))

(fn SetWeapon
  (Default|SetWeapon (Variables|Default|GetPlayer) (Utilities|Array|Get(acopy) (Variables|Default|GetWeapons) (Variables|Default|GetNextWeaponIndex)))
  (bind _output_get (Variables|Default|SetNextWeaponIndex (+ (Variables|Default|GetNextWeaponIndex) 1)))
  (if (>= _output_get (Utilities|Array|Length (Variables|Default|GetWeapons)))
    (Variables|Default|SetNextWeaponIndex 0)))