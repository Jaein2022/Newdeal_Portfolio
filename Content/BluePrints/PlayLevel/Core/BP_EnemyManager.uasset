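; BP_EnemyManager drives timed enemy spawning in the play level.
; The construction script caches all BP_SpawnPoint actors in the SpawnPoints array, and an older copy of that logic sits disconnected in the EventGraph.
; Tick accumulates time, calls Spawn on a random point when the timer expires, then rerolls the delay within a fixed range.
; The random index assumes five spawn points instead of using the array length.
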(event EventBeginPlay)

(event EventTick
  (params (DeltaSeconds :type Float%20%28single-precision%29))
  ;[0.1406 0.1406 0.1406] 일정 시간마다 랜덤한 스폰 포인트에서 랜덤한 시간마다 적 생성
  (bind _output_get (Variables|Default|SetAccSpawnTime (+ DeltaSeconds (Variables|Default|GetAccSpawnTime))))
  (if (>= _output_get (Variables|Default|GetNextSpawnTime))
    (Default|Spawn (Utilities|Array|Get(acopy) (Variables|Default|GetSpawnPoints) (Math|Random|RandomInteger 5)))
    (Variables|Default|SetAccSpawnTime 0.0)
    (Variables|Default|SetNextSpawnTime (Math|Random|RandomFloatinRange 15.0 2e+01))))

(fn ConstructionScript
  (bind _outactors (Actor|GetAllActorsOfClass "/Game/BluePrints/PlayLevel/Enemy/BP_SpawnPoint.BP_SpawnPoint_C"))
  (Utilities|Array|Resize (Variables|Default|GetSpawnPoints) (Utilities|Array|Length _outactors))
  (Variables|Default|SetSpawnPoints _outactors))