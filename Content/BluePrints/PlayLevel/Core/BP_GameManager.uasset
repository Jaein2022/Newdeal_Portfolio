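; BP_GameManager is a play-level hub that holds the enemy, sound, player and weapon managers and exposes a getter for each.
; The enemy and weapon getters cast the child actor of their components to the manager class, while the sound and player getters return their members directly.
; The event graph and construction script are empty, so this Blueprint contains only accessor logic.
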(event EventBeginPlay)

(event Collision|EventActorBeginOverlap
  (params (OtherActor :type Actor%20Object%20Reference)))

(event EventTick
  (params (DeltaSeconds :type Float%20%28single-precision%29)))

(fn ConstructionScript)

(fn GetEnemyManager
  (bind _asbp_enemy_manager (Utilities|Casting|CastToBP_EnemyManager (Variables|/Script/Engine.ChildActorComponent|GetChildActor (Variables|Default|GetBP_EnemyManager))))
  (return _asbp_enemy_manager))

(fn GetSoundManager
  (return (Variables|Default|GetBP_SoundManager)))

(fn GetPlayerManager
  (return (Variables|Default|GetBP_PlayerManager)))

(fn GetWeaponManager
  (bind _asbp_weapon_manager (Utilities|Casting|CastToBP_WeaponManager (Variables|/Script/Engine.ChildActorComponent|GetChildActor (Variables|Default|GetBP_WeaponManager))))
  (return _asbp_weapon_manager))