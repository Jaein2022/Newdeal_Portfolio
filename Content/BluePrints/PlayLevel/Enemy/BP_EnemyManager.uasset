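; BP_EnemyManager drives timed enemy spawning in the play level.
; On BeginPlay it gathers every BP_SpawnPoint actor in the world into an array.
; Tick accumulates delta time and, once the next spawn time is reached, calls Spawn on a randomly chosen point, then resets the timer and rolls a new random delay within a fixed range.
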(event EventBeginPlay
  ;[0.1406 0.1406 0.1406] 게임내에 있는 스폰 포인트를 배열로 저장
  (bind _outactors (Actor|GetAllActorsOfClass "/Game/BluePrints/PlayLevel/Enemy/BP_SpawnPoint.BP_SpawnPoint_C"))
  (Utilities|Array|Resize (Variables|Default|GetSpawnPoints) (Utilities|Array|Length _outactors))
  (Variables|Default|SetSpawnPoints _outactors))

(event EventTick
  (params (DeltaSeconds :type Float%20%28single-precision%29))
  (bind _spawnpoints (Variables|Default|GetSpawnPoints))
  ;[0.1406 0.1406 0.1406] 일정 시간마다 랜덤한 스폰 포인트에서 랜덤한 시간마다 적 생성
  (bind _output_get (Variables|Default|SetAccSpawnTime (+ DeltaSeconds (Variables|Default|GetAccSpawnTime))))
  (if (>= _output_get (Variables|Default|GetNextSpawnTime))
    (Default|Spawn (Utilities|Array|Get(acopy) _spawnpoints (Math|Random|RandomInteger (Utilities|Array|Length _spawnpoints))))
    (Variables|Default|SetAccSpawnTime 0.0)
    (Variables|Default|SetNextSpawnTime (Math|Random|RandomFloatinRange 5.0 1e+01))))

(fn ConstructionScript)