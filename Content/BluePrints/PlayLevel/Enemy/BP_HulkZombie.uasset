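; BP_HulkZombie is a slow, armored zombie enemy that overrides damage handling from its parent.
; Armor reduces body-shot damage, sparking a metallic effect when fully absorbed, while headshots and explosions bypass it and explosions add a DOT stack.
; Surviving hits play montages, with headshots and explosions halting movement until MoveToPlayer resumes it.
; Death awards the VR player rocket ammo, with a larger reward for headshots or a random chance.
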(event Custom|PlayArmorHitEffect
  (params (HitLocation :type Vector))
  (bind _armorhiteffect (Variables|Default|GetArmorHitEffect))
  (Transformation|SetWorldLocation _armorhiteffect HitLocation false true)
  (Components|Activation|Activate _armorhiteffect true)
  (bind _returnvalue (Audio|SpawnSoundatLocation "/Game/ZombieAsset/HulkZombie/407349__forthehorde68__fx_metallic_hit.407349__forthehorde68__fx_metallic_hit" HitLocation "0, 0, 0" 1.25 6.0 0.27 "/Game/MilitaryWeapSilver/Sound/Attenuation/ProjectileImpact_att.ProjectileImpact_att" 0))
  (Audio|Components|Audio|StopDelayed _returnvalue 0.5))

(event EventBeginPlay
  (|CallParentFunction)
  (Variables|/Script/Engine.CharacterMovementComponent|SetMaxWalkSpeed (Variables|Character|GetCharacterMovement) 2e+02))

(event Collision|EventActorBeginOverlap
  (params (OtherActor :type Actor%20Object%20Reference)))

(event EventTick
  (params (DeltaSeconds :type Float%20%28single-precision%29))
  (|CallParentFunction DeltaSeconds) ; This node is disabled and will not be called.\nDrag off pins to build functionality.
)

(event EventOnDamaged
  (params (InDamage :type Integer) (IsHeadShot :type Boolean) (IsExplosion :type Boolean) (HitLocation :type Vector :default "0, 0, 0"))
  (bind _hitanimmontages (Variables|Default|GetHitAnimMontages))
  (bind _armor (Variables|Default|GetArmor))
  (bind _returnvalue (- InDamage _armor))
  (if (and (not IsHeadShot) (not IsExplosion))
    (if (> _returnvalue 0)
      (Variables|Default|SetHP (- (Variables|Default|GetHP) _returnvalue))
      (if (<= (stale _output_get) 0) :!label _label
        ;[0.1406 0.1406 0.1406] 죽었을때
        (if (not (Variables|Default|GetIsDead))
          (Variables|Default|SetIsDead true)
          (CallFunction|AddPlayerAmmo IsHeadShot)
          (CallFunction|OnDead))
        (else
          ;[0.1406 0.1406 0.1406] 피격시
          (if IsExplosion
            (Components|Movement|StopMovementImmediately (Variables|Character|GetCharacterMovement))
            (Animation|Montage|PlayMontage (Variables|Character|GetMesh) (Variables|Default|GetBigHitAnimMontage) 2.0
              (:OnCompleted
                (CallFunction|MovetoPlayer)))
            (elif IsHeadShot
              (CallFunction|PlayFleshHitEffect true HitLocation)
              (Components|Movement|StopMovementImmediately (Variables|Character|GetCharacterMovement))
              (Animation|Montage|PlayMontage (Variables|Character|GetMesh) (Variables|Default|GetHeadshotAnimMontage) 1.75
                (:OnCompleted
                  (CallFunction|MovetoPlayer)))
              (else
                (CallFunction|PlayFleshHitEffect false HitLocation)
                (Animation|Montage|PlayMontage (Variables|Character|GetMesh) (Utilities|Array|Get(acopy) _hitanimmontages (Math|Random|RandomInteger (Utilities|Array|Length _hitanimmontages))) 1.5))))))
      (else
        (CallFunction|PlayArmorHitEffect HitLocation)))
    (else
      (bind _output_get (Variables|Default|SetHP (- (Variables|Default|GetHP) InDamage)))
      (if IsExplosion
        (Math|Integer|IncrementInt (Variables|Default|GetDOTStackCount)
          (:%20%20
            (goto _label)))
        (else
          (goto _label))))))

(event EventAddPlayerAmmo
  (params (IsHeadShot :type Boolean))
  (bind _asbp_player_vr (Utilities|Casting|CastToBP_Player_VR (Variables|Default|GetTargetPlayer)))
  (if IsHeadShot
    (Default|AddAmmo _asbp_player_vr "NewEnumerator2" 2)
    (Development|PrintString "Rocket: 2" true true "(R=0.000000,G=0.660000,B=1.000000,A=1.000000)" 1e+01)
    (elif (Math|Random|RandomBoolwithWeight 0.25)
      (Default|AddAmmo _asbp_player_vr "NewEnumerator2" 2)
      (Development|PrintString "Rocket: 2" true true "(R=0.000000,G=0.660000,B=1.000000,A=1.000000)" 1e+01)
      (else
        (Default|AddAmmo _asbp_player_vr "NewEnumerator2" 1)
        (Development|PrintString "Rocket: 1" true true "(R=0.000000,G=0.660000,B=1.000000,A=1.000000)" 1e+01)))))

(fn ConstructionScript
  (|CallParentFunction))