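; Prisoner zombie enemy that approaches its target player and attacks from a randomized long stand-off distance.
; MovetoPlayer runs AI Move To, then line-traces toward the player, ignoring other enemies; a blocked trace shrinks the distance and retries, while a clear hit enables attacking.
; TryAttack plays a random montage, then accumulates delta time until the cooldown re-arms it.
; The montage notify only prints a debug string, with no damage logic here.
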(event EventBeginPlay
  (|CallParentFunction)
  (Variables|Default|SetAttackDistance (Math|Random|RandomFloatinRange 1.8e+03 2.2e+03)))

(event Collision|EventActorBeginOverlap
  (params (OtherActor :type Actor%20Object%20Reference)))

(event EventTick
  (params (DeltaSeconds :type Float%20%28single-precision%29))
  (|CallParentFunction DeltaSeconds) ; This node is disabled and will not be called.\nDrag off pins to build functionality.
)

(event EventTryAttack
  (bind _attackanimmontages (Variables|Default|GetAttackAnimMontages))
  (if (Variables|Default|GetbCanAttack)
    (Variables|Default|SetbCanAttack false)
    (Animation|Montage|PlayMontage (Variables|Character|GetMesh) (Utilities|Array|Get(acopy) _attackanimmontages (Math|Random|RandomInteger (Utilities|Array|Length _attackanimmontages)))
      (:OnNotifyBegin
        (Development|PrintString "Attack!")))
    (else
      (bind _output_get (Variables|Default|SetAttackAccTime (+ (Variables|Default|GetAttackAccTime) (Utilities|Time|GetWorldDeltaSeconds))))
      (if (>= _output_get (Variables|Default|GetAttackCoolTime))
        (Variables|Default|SetAttackAccTime (- (Variables|Default|GetAttackAccTime) (Variables|Default|GetAttackCoolTime)))
        (Variables|Default|SetbCanAttack true)))))

(event EventMovetoPlayer
  (bind _returnvalue (Transformation|GetActorLocation))
  (bind _returnvalue_2 (Transformation|GetActorLocation))
  (bind _targetplayer (Variables|Default|GetTargetPlayer))
  (bind _returnvalue_3 (Transformation|GetActorLocation _targetplayer))
  (bind _returnvalue_4 (Math|Rotator|FindLookatRotation _returnvalue_2 _returnvalue_3))
  (AI|AIMoveTo self "0, 0, 0" (Variables|Default|GetTargetPlayer) (Variables|Default|GetAttackDistance) false
    (:OnSuccess
      (Transformation|SetActorRotation _returnvalue_4)
      (bind _outactors (Actor|GetAllActorsOfClass "/Game/BluePrints/PlayLevel/Enemy/BP_EnemyCharacter_Base.BP_EnemyCharacter_Base_C"))
      (bind _outhit (Collision|LineTraceByChannel _returnvalue (+ _returnvalue (* (Math|Vector|GetForwardVector _returnvalue_4) (Variables|Default|GetAttackDistance))) "TraceTypeQuery2" false _outactors "ForDuration" true "(R=1.000000,G=0.000000,B=0.000000,A=1.000000)" "(R=0.000000,G=1.000000,B=0.000000,A=1.000000)" 2.0))
      (bind _asbp_player (Utilities|Casting|CastToBP_Player (.hitactor _outhit))
        (:then
          (if (== _asbp_player (Variables|Default|GetTargetPlayer))
            (Variables|Default|SetbCanAttack true)
            (Variables|Default|SetIsArrived true)
            (else
              (Variables|Default|SetAttackDistance (- (Variables|Default|GetAttackDistance) 2e+02) :!label _label)
              (CallFunction|MovetoPlayer))))
        (:CastFailed
          (goto _label))))))

(fn ConstructionScript
  (|CallParentFunction))