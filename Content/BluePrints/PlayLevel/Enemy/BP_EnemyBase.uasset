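; Base enemy actor that uses AI MoveTo toward the player pawn on BeginPlay and takes damage through a custom Damaged event.
; Hits pause the movement timeline and briefly set a damaged flag, while zero HP marks death and destroys the actor after a delay.
; Tick snaps head and body collision to mesh sockets.
; Spline-path timeline movement and cooldown montage attacks that damage BP_Player on a notify are present but disconnected.
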(event Custom|Damaged
  (params (InDamage :type Integer))
  ;[0.1406 0.1406 0.1406] 데미지 처리 ( 나중에 Anydamage로 변경?)
  (bind _output_get (Variables|Default|SetHP (- (Variables|Default|GetHP) InDamage)))
  (if (<= _output_get 0)
    ;;[0.1406 0.1406 0.1406] 죽었을때
    (Variables|Default|SetbIsMove false)
    (Variables|Default|SetbIsDead true)
    (Audio|Components|Audio|Stop (Variables|Default|GetEnemyMoveTimeLine))
    (Utilities|FlowControl|Delay 3.0)
    (Actor|DestroyActor)
    (else
      ;;[0.1406 0.1406 0.1406] 피격시
      (Variables|Default|SetbIsDamaged true)
      (Audio|Components|Audio|Stop (Variables|Default|GetEnemyMoveTimeLine))
      (Utilities|FlowControl|Delay 2.0)
      (Variables|Default|SetbIsDamaged false)
      (if (not (Variables|Default|GetbIsDead))
        (Audio|Components|Audio|Play (Variables|Default|GetEnemyMoveTimeLine))))))

(event EventBeginPlay
  (AI|AIMoveTo self "0, 0, 0" (Game|Player|GetPlayerPawn 0) 5.0 false))

(event EventTick
  (params (DeltaSeconds :type Float%20%28single-precision%29))
  (Utilities|FlowControl|Sequence
    (:then_0
      ;[0.1406 0.1406 0.1406] 머리랑 몸통 콜리전이 머리와 몸통 소켓을 따라다니게(필요할까?)
      (Transformation|SetWorldLocation (Variables|Default|GetBody) (Transformation|GetSocketLocation (Variables|Default|GetSkeletalMesh) "BodyCollisionSocket") false false)
      (Transformation|SetWorldLocation (Variables|Default|GetHead) (Transformation|GetSocketLocation (Variables|Default|GetSkeletalMesh) "HeadCollisionSocket") false false))))

(fn ConstructionScript)

(fn SetTimeLinePlayrate
  (params (InPlayrate :type Float%20%28double-precision%29))
  (Components|Timeline|SetPlayRate (Variables|Default|GetEnemyMoveTimeLine) InPlayrate))