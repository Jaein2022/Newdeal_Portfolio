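; BP_CopZombie is a zombie enemy variant that charges the player and rewards rifle ammo.
; Tick extends the parent's behavior: when the target comes within horizontal range, it permanently doubles walk speed and plays a charge sound attached to its head.
; The sound stops once the zombie is dead.
; AddPlayerAmmo gives the VR player rifle ammo, with a larger amount for headshots, and prints a debug message.
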(event EventBeginPlay
  (|CallParentFunction)
  (bind _returnvalue (Audio|SpawnSoundAttached (Variables|Default|GetChargeSound) (Variables|Default|GetHead) "None" "0, 0, 0" "0, 0, 0" "KeepRelativeOffset" false 1.0 1.0 0.0 0 0 false))
  (bind _output_get (Variables|Default|SetChargingSoundComponent _returnvalue))
  (Audio|Components|Audio|Stop _output_get))

(event Collision|EventActorBeginOverlap
  (params (OtherActor :type Actor%20Object%20Reference)))

(event EventTick
  (params (DeltaSeconds :type Float%20%28single-precision%29))
  (bind _charactermovement (Variables|Character|GetCharacterMovement))
  (bind _chargingsoundcomponent (Variables|Default|GetChargingSoundComponent))
  (|CallParentFunction DeltaSeconds)
  (Utilities|FlowControl|Sequence
    (:then_0
      (if (<= (Class|Actor|GetSquaredHorizontalDistanceto (Variables|Default|GetTargetPlayer)) (Math|Float|Square 1.75e+03))
        (if (not (Variables|Default|GetIsCharging))
          (Audio|Components|Audio|Play (Variables|Default|GetChargingSoundComponent) 0.0)
          (Variables|Default|SetIsCharging true)
          (Variables|/Script/Engine.CharacterMovementComponent|SetMaxWalkSpeed _charactermovement (* 2.0 (Variables|/Script/Engine.CharacterMovementComponent|GetMaxWalkSpeed _charactermovement))))))
    (:then_1
      (if (and (Variables|Default|GetIsCharging) (Variables|Default|GetIsDead))
        (if (Audio|Components|Audio|IsPlaying _chargingsoundcomponent)
          (Audio|Components|Audio|Stop _chargingsoundcomponent))))))

(event EventMovetoPlayer
  (|CallParentFunction))

(event EventAddPlayerAmmo
  (params (IsHeadShot :type Boolean))
  (bind _asbp_player_vr (Utilities|Casting|CastToBP_Player_VR (Variables|Default|GetTargetPlayer)))
  (if IsHeadShot
    (Default|AddAmmo _asbp_player_vr "NewEnumerator1" 30)
    (Development|PrintString "Rifle: 30" true true "(R=0.000000,G=0.660000,B=1.000000,A=1.000000)" 1e+01)
    (else
      (Default|AddAmmo _asbp_player_vr "NewEnumerator1" 15)
      (Development|PrintString "Rifle: 15" true true "(R=0.000000,G=0.660000,B=1.000000,A=1.000000)" 1e+01))))

(fn ConstructionScript
  (|CallParentFunction))