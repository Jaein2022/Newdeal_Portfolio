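; Base enemy character that chases the player, attacks with random montages on a cooldown and deals damage on the montage notify.
; Hits on it play flesh effects and reactions, with double damage for headshots and stacking burn damage over time from explosions.
; Head and body components attach to mesh sockets.
; Death disables mesh collision, scales out any fire and destroys the actor, while kills by direct hit also award rifle ammo.
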(event Custom|MoveToPlayer
  (AI|AIMoveTo self "0, 0, 0" (Variables|Default|GetTargetPlayer) (Variables|Default|GetAttackDistance) false
    (:OnSuccess
      (Variables|Default|SetbCanAttack true)
      (Variables|Default|SetIsArrived true))))

(event Custom|OnDamaged
  (params (InDamage :type Integer) (IsHeadShot :type Boolean) (IsExplosion :type Boolean) (HitLocation :type Vector))
  (bind _hitanimmontages (Variables|Default|GetHitAnimMontages))
  ;[0.1406 0.1406 0.1406] 데미지 처리
  (if IsHeadShot
    (Variables|Default|SetHP (- (Variables|Default|GetHP) (* InDamage 2)))
    (else
      (bind _output_get (Variables|Default|SetHP (- (Variables|Default|GetHP) InDamage)))))
  (if IsExplosion
    (Math|Integer|IncrementInt (Variables|Default|GetDOTStackCount)
      (:%20%20
        _)))
  (Components|Movement|StopMovementImmediately (Variables|Character|GetCharacterMovement))
  (if (<= _output_get 0)
    ;;[0.1406 0.1406 0.1406] 죽었을때
    (if (not (Variables|Default|GetIsDead))
      (Variables|Default|SetIsDead true)
      (CallFunction|PlayFleshHitEffect IsHeadShot HitLocation)
      (CallFunction|AddPlayerAmmo IsHeadShot)
      (CallFunction|OnDead))
    (else
      ;;[0.1406 0.1406 0.1406] 피격시
      (CallFunction|PlayFleshHitEffect IsHeadShot HitLocation)
      (Animation|Montage|PlayMontage (Variables|Character|GetMesh) (Utilities|Array|Get(acopy) _hitanimmontages (Math|Random|RandomInteger (Utilities|Array|Length _hitanimmontages))) 2.0
        (:OnCompleted
          (CallFunction|MovetoPlayer))))))

(event Custom|TryAttack
  (bind _attackanimmontages (Variables|Default|GetAttackAnimMontages))
  ;[0.1406 0.1406 0.1406] 공격
  (if (Variables|Default|GetbCanAttack)
    (Variables|Default|SetbCanAttack false)
    (Animation|Montage|PlayMontage (Variables|Character|GetMesh) (Utilities|Array|Get(acopy) _attackanimmontages (Math|Random|RandomInteger (Utilities|Array|Length _attackanimmontages)))
      (:OnNotifyBegin
        (bind _asbp_player_vr (Utilities|Casting|CastToBP_Player_VR (Variables|Default|GetTargetPlayer)))
        (Default|GetDamage _asbp_player_vr (Variables|Default|GetDamage))))
    (else
      (bind _output_get (Variables|Default|SetAttackAccTime (+ (Variables|Default|GetAttackAccTime) (Utilities|Time|GetWorldDeltaSeconds))))
      (if (>= _output_get (Variables|Default|GetAttackCoolTime))
        (Variables|Default|SetAttackAccTime (- (Variables|Default|GetAttackAccTime) (Variables|Default|GetAttackCoolTime)))
        (Variables|Default|SetbCanAttack true)))))

(event Custom|OnDead
  (bind _burningeffect (Variables|Default|GetBurningEffect))
  (Utilities|FlowControl|Sequence
    (:then_0
      (Collision|SetCollisionEnabled (Variables|Character|GetMesh) "NoCollision"))
    (:then_1
      (if (Components|Activation|IsActive (Variables|Default|GetBurningEffect))
        (bind _firescale (Timeline|Timeline PlayFromStart)
          (:Update
            (Transformation|SetRelativeScale3D _burningeffect _firescale))
          (:Finished
            (Components|Activation|Deactivate _burningeffect)))))
    (:then_2
      (Utilities|FlowControl|Delay 3.0)
      (Actor|DestroyActor))))

(event Custom|AddPlayerAmmo
  (params (IsHeadShot :type Boolean))
  (bind _asbp_player_vr (Utilities|Casting|CastToBP_Player_VR (Variables|Default|GetTargetPlayer)))
  (if IsHeadShot
    (Default|AddAmmo _asbp_player_vr "NewEnumerator1" 10)
    (Development|PrintString "Rifle: 10" true true "(R=0.000000,G=0.660000,B=1.000000,A=1.000000)" 1e+01)
    (else
      (Default|AddAmmo _asbp_player_vr "NewEnumerator1" 5)
      (Development|PrintString "Rifle: 5" true true "(R=0.000000,G=0.660000,B=1.000000,A=1.000000)" 1e+01))))

(event Custom|PlayFleshHitEffect
  (params (IsHeadShot :type Boolean) (HitLocation :type Vector))
  (bind _bodyhiteffect (Variables|Default|GetBodyHitEffect))
  (bind _headhiteffect (Variables|Default|GetHeadHitEffect))
  (bind _fleshhitsounds (Variables|Default|GetFleshHitSounds))
  (bind _returnvalue (Utilities|Array|Length _fleshhitsounds))
  (bind _returnvalue_2 (Math|Random|RandomInteger _returnvalue))
  (bind _output (Utilities|Array|Get(acopy) _fleshhitsounds _returnvalue_2))
  (if IsHeadShot
    (Audio|PlaySoundatLocation _output HitLocation "0, 0, 0" 2.0 1.0 0.0 "/Game/MilitaryWeapSilver/Sound/Attenuation/ProjectileImpact_att.ProjectileImpact_att" 0 0 0)
    (Transformation|SetWorldLocation _headhiteffect HitLocation false true)
    (Components|Activation|Activate _headhiteffect true)
    (else
      (Audio|PlaySoundatLocation _output HitLocation "0, 0, 0" 1.0 1.0 0.0 "/Game/MilitaryWeapSilver/Sound/Attenuation/ProjectileImpact_att.ProjectileImpact_att" 0 0 0)
      (Transformation|SetWorldLocation _bodyhiteffect HitLocation false true)
      (Components|Activation|Activate _bodyhiteffect true))))

(event EventBeginPlay
  (bind _asbp_player (Utilities|Casting|CastToBP_Player (Game|Player|GetPlayerPawn 0)))
  (Variables|Default|SetTargetPlayer _asbp_player)
  (CallFunction|MovetoPlayer)
  (Components|Activation|Deactivate (Variables|Default|GetBurningEffect)))

(event EventTick
  (params (DeltaSeconds :type Float%20%28single-precision%29))
  (bind _burningeffect (Variables|Default|GetBurningEffect))
  (bind _burningeffect_2 (Variables|Default|GetBurningEffect))
  (if (not (Variables|Default|GetIsDead))
    (Utilities|FlowControl|Sequence
      (:then_0
        (if (> (Variables|Default|GetDOTStackCount) 0)
          (CallFunction|Burn)
          (if (not (Components|Activation|IsActive _burningeffect))
            (Components|Activation|Activate _burningeffect true))
          (elif (Components|Activation|IsActive _burningeffect_2)
            (Components|Activation|Deactivate _burningeffect_2))))
      (:then_1
        (if (Variables|Default|GetIsArrived)
          (CallFunction|TryAttack))))
    (else
      (Components|Movement|StopMovementImmediately (Variables|Character|GetCharacterMovement)))))

(fn ConstructionScript
  (Transformation|AttachComponentToComponent (Variables|Default|GetHead) (Variables|Character|GetMesh) "HeadSocket" "KeepRelative" "KeepRelative" "KeepRelative" true)
  (Transformation|AttachComponentToComponent (Variables|Default|GetBody) (Variables|Character|GetMesh) "HipsSocket" "KeepWorld" "KeepWorld" "KeepRelative" true)
  (Transformation|AttachComponentToComponent (Variables|Default|GetBurningEffect) (Variables|Character|GetMesh) "HipsSocket" "KeepRelative" "SnapToTarget" "KeepRelative" true))

(fn GetIsAttack
  (return (Variables|Default|GetbCanAttack)))

(fn Burn
  (bind _output_get (Variables|Default|SetBurningAccTime (+ (Variables|Default|GetBurningAccTime) (Utilities|Time|GetWorldDeltaSeconds))))
  (if (>= _output_get 1.0)
    (Variables|Default|SetBurningAccTime (- (Variables|Default|GetBurningAccTime) 1.0))
    (bind _output_get_2 (Variables|Default|SetHP (- (Variables|Default|GetHP) (* (Variables|Default|GetBurningDamagePerSecond) (Variables|Default|GetDOTStackCount)))))
    (if (<= _output_get_2 0)
      (if (not (Variables|Default|GetIsDead))
        (Variables|Default|SetIsDead true)
        (CallFunction|OnDead)))))