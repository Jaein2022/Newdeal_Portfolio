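; BP_PlayerTitle is the title-level VR player, using Stage tracking origin and left and right widget interaction pointers for menu UI.
; Menu-select input on each hand presses and releases a simulated left mouse button on that hand's WidgetInteraction component.
; Both Niagara beams are shown at BeginPlay, but Tick updates only the left, feeding it a two-point array from the pointer origin to its full interaction distance.
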(event Input|EnhancedActionEvents|EnhancedInputActionIA_MenuSelectLeft
  (params (ActionValue :type Boolean) (ElapsedSeconds :type Float%20%28double-precision%29) (TriggeredSeconds :type Float%20%28double-precision%29) (InputAction :type Input%20Action%20Object%20Reference :default "/Game/BluePrints/PlayLevel/Player/Input/Action/VR/IA_MenuSelectLeft.IA_MenuSelectLeft"))
  ;[0.4219 1 0.3112] MenuUI 연동
  (:Started
    (Class|WidgetInteractionComponent|PressPointerKey (Variables|Default|GetWidgetInteractionLeft) "LeftMouseButton"))
  (:Completed
    (Class|WidgetInteractionComponent|ReleasePointerKey (Variables|Default|GetWidgetInteractionLeft) "LeftMouseButton")))

(event Input|EnhancedActionEvents|EnhancedInputActionIA_MenuSelectRight
  (params (ActionValue :type Boolean) (ElapsedSeconds :type Float%20%28double-precision%29) (TriggeredSeconds :type Float%20%28double-precision%29) (InputAction :type Input%20Action%20Object%20Reference :default "/Game/BluePrints/PlayLevel/Player/Input/Action/VR/IA_MenuSelectRight.IA_MenuSelectRight"))
  ;[0.4219 1 0.3112] MenuUI 연동
  (:Started
    (Class|WidgetInteractionComponent|PressPointerKey (Variables|Default|GetWidgetInteractionRight) "LeftMouseButton"))
  (:Completed
    (Class|WidgetInteractionComponent|ReleasePointerKey (Variables|Default|GetWidgetInteractionRight) "LeftMouseButton")))

(event EventBeginPlay
  (|CallParentFunction)
  (Class|HeadMountedDisplayFunctionLibrary|SetTrackingOrigin "Stage")
  (Rendering|SetVisibility (Variables|Default|GetLeftWidgetNiagara) true false)
  (Rendering|SetVisibility (Variables|Default|GetRightWidgetNiagara) true false))

(event EventTick
  (params (DeltaSeconds :type Float%20%28single-precision%29))
  (CallFunction|WidgetTraceNiagara (Variables|Default|GetWidgetInteractionLeft) (Variables|Default|GetLeftWidgetNiagara)))

(fn ConstructionScript
  (|CallParentFunction))

(fn WidgetTraceNiagara
  (params (InWidgetInteraction :type Widget%20Interaction%20Component%20Object%20Reference) (InNiagaraSystem :type Niagara%20Component%20Object%20Reference))
  (bind _localpointarray (LocalVariables|GetLocalPointArray))
  (bind _returnvalue (Transformation|GetWorldLocation InWidgetInteraction))
  (Utilities|Array|Resize _localpointarray 2)
  (Utilities|Array|SetArrayElem _localpointarray 0 _returnvalue)
  (Utilities|Array|SetArrayElem (LocalVariables|GetLocalPointArray) 1 (+ (* (Class|KismetMathLibrary|MatrixGetUnitAxis (Math|Transform|ToMatrix(Transform) (Transformation|GetWorldTransform InWidgetInteraction)) "X") (Variables|/Script/UMG.WidgetInteractionComponent|GetInteractionDistance InWidgetInteraction)) _returnvalue))
  (Class|NiagaraDataInterfaceArrayFunctionLibrary|SetNiagaraArrayVector InNiagaraSystem "User.InPointArray" (LocalVariables|GetLocalPointArray)))