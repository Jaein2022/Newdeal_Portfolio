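; BP_Light is an effect actor whose two point lights react to enemy characters passing through its Box trigger.
; Both lights start hidden on BeginPlay.
; A BP_EnemyCharacter_Base entering the box shows PointLight for a few seconds.
; One leaving it briefly flashes PointLight2 in red, with each light hidden again after a Delay.
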(event OnComponentBeginOverlap(Box)
  (params (OverlappedComponent :type Primitive%20Component%20Object%20Reference) (OtherActor :type Actor%20Object%20Reference) (OtherComp :type Primitive%20Component%20Object%20Reference) (OtherBodyIndex :type Integer) (bFromSweep :type Boolean) (SweepResult :type Hit%20Result%20Structure%20%28by%20ref%29))
  (Utilities|Casting|CastToBP_EnemyCharacter_Base OtherActor)
  (Rendering|SetVisibility (Variables|Default|GetPointLight) true false)
  (Utilities|FlowControl|Delay 3.0)
  (Rendering|SetVisibility (Variables|Default|GetPointLight) false false))

(event OnComponentEndOverlap(Box)
  (params (OverlappedComponent :type Primitive%20Component%20Object%20Reference) (OtherActor :type Actor%20Object%20Reference) (OtherComp :type Primitive%20Component%20Object%20Reference) (OtherBodyIndex :type Integer))
  (Utilities|Casting|CastToBP_EnemyCharacter_Base OtherActor)
  (Rendering|SetVisibility (Variables|Default|GetPointLight2) true false)
  (Rendering|Components|Light|SetLightColor (Variables|Default|GetPointLight2) "(R=1.000000,G=0.000000,B=0.035352,A=1.000000)" true)
  (Utilities|FlowControl|Delay 0.3)
  (Rendering|SetVisibility (Variables|Default|GetPointLight2) false false))

(event EventBeginPlay
  (Rendering|SetVisibility (Variables|Default|GetPointLight) false false)
  (Rendering|SetVisibility (Variables|Default|GetPointLight2) false false))

(event Collision|EventActorBeginOverlap
  (params (OtherActor :type Actor%20Object%20Reference)))

(event EventTick
  (params (DeltaSeconds :type Float%20%28single-precision%29)))

(fn ConstructionScript)